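; BP_Basket is the basket actor in the Apple Picker game that catches objects to score.
; On BeginPlay it caches GS_GameState and stores its bottom, middle and top meshes in an array.
; Any actor that begins overlapping its Box is destroyed without a type check, then the game state updates the score.
; Move and DestroyMesh events reposition the root without sweep and remove a given mesh component.
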(event OnComponentBeginOverlap(Box)
  (params (OverlappedComponent :type Primitive%20Component%20Object%20Reference) (OtherActor :type Actor%20Object%20Reference) (OtherComp :type Primitive%20Component%20Object%20Reference) (OtherBodyIndex :type Integer) (bFromSweep :type Boolean) (SweepResult :type Hit%20Result%20Structure%20%28by%20ref%29))
  (Actor|DestroyActor OtherActor)
  (Default|UpdateGameScore (Variables|Default|GetGame%20State)))

(event Custom|Move
  (params (New%20Position :type Vector))
  (Transformation|SetWorldLocation (Variables|Default|GetDefaultSceneRoot) New%20Position false false))

(event Custom|DestroyMesh
  (params (Mesh :type Static%20Mesh%20Component%20Object%20Reference))
  (Components|DestroyComponent Mesh))

(event EventBeginPlay
  (bind _basket_meshes (Variables|Default|GetBasket%20Meshes))
  (bind _asgs_game_state (Utilities|Casting|CastToGS_GameState (Game|GetGameState)))
  (Utilities|IsValid _asgs_game_state
    (:Is%20Valid
      (Variables|Default|SetGame%20State _asgs_game_state)
      (Utilities|Array|Add _basket_meshes (Variables|Default|GetBottom%20Mesh))
      (Utilities|Array|Add _basket_meshes (Variables|Default|GetMiddle%20Mesh))
      (Utilities|Array|Add _basket_meshes (Variables|Default|GetTop%20Mesh)))))

(fn ConstructionScript)