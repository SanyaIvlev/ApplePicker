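; Player controller for ApplePicker that lets the mouse slide the player's basket horizontally.
; On begin play it caches the controlled pawn as a BP_Basket, shows the cursor and adds the WBP_MatchInfo widget to the viewport.
; Each tick it deprojects the mouse screen position to world space and passes only the X to the basket's Move, keeping the basket's current Y and Z.
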(event EventTick
  (params (DeltaSeconds :type Float%20%28single-precision%29))
  (bind (_locationx _locationy) (Game|Player|GetMousePosition))
  (bind _basket (Variables|Default|GetBasket))
  (bind _basket_2 (Variables|Default|GetBasket))
  (bind _defaultsceneroot (Variables|/Game/ApplePicker/Blueprints/BP_Basket.BP_Basket_C|GetDefaultSceneRoot _basket_2))
  (bind _returnvalue (Transformation|GetWorldLocation _defaultsceneroot))
  (Utilities|IsValid _basket
    (:Is%20Valid
      (Default|Move _basket (Math|Vector|MakeVector (.x (.WorldLocation (Class|PlayerController|DeprojectScreenPositiontoWorld _locationx _locationy))) (.y _returnvalue) (.z _returnvalue))))))

(event EventBeginPlay
  (CallFunction|InitializeVariables)
  (Variables|Default|SetbShowMouseCursor true)
  (bind _returnvalue (Game|ConstructObjectfromClass "/Game/ApplePicker/Blueprints/WBP_MatchInfo.WBP_MatchInfo_C"))
  (UserInterface|Viewport|AddtoViewport _returnvalue 0))

(fn ConstructionScript)

(fn InitializeVariables
  (bind _asbp_basket (Utilities|Casting|CastToBP_Basket (Pawn|GetControlledPawn)))
  (Utilities|IsValid _asbp_basket
    (:Is%20Valid
      (Variables|Default|SetBasket _asbp_basket))))