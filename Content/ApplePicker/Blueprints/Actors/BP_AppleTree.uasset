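; BP_AppleTree is the apple tree actor for ApplePicker, sliding along the X axis and spawning BP_Apple actors.
; Tick moves the root by MovementVector and points it back inward once it passes either LeftAndRightEdge bound.
; BeginPlay starts two looping timers, named for random rotation checks and apple drops.
; TryRotateRandomly changes MovementVector by chance, and DropApple spawns an apple at the root's transform.
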(event EventBeginPlay
  (Utilities|Time|SetTimerbyEvent (EventDispatchers|CreateEvent :!event TryRotateRandomly) (Variables|Default|GetRandom%20Rotation%20Check%20Delay) true)
  (Utilities|Time|SetTimerbyEvent (EventDispatchers|CreateEvent :!event DropApple) (Variables|Default|GetAppleDropDelay) true false 2.0))

(event EventTick
  (params (DeltaSeconds :type Float%20%28single-precision%29))
  (CallFunction|Move DeltaSeconds)
  (CallFunction|TryRotateonEdge))

(fn ConstructionScript)

(fn Move
  (params (Delta%20Seconds :type Float%20%28double-precision%29))
  (bind _defaultsceneroot (Variables|Default|GetDefaultSceneRoot))
  (bind _returnvalue (Transformation|GetWorldLocation _defaultsceneroot))
  (bind (_x _y _z) (Math|Vector|BreakVector _returnvalue))
  (Transformation|SetWorldLocation (Variables|Default|GetDefaultSceneRoot) (Math|Vector|MakeVector (+ (* Delta%20Seconds (Variables|Default|GetMovementVector)) _x) _y _z) false false))

(fn TryRotateonEdge
  (if (< (.x (Transformation|GetWorldLocation (Variables|Default|GetDefaultSceneRoot))) (* (Variables|Default|GetLeftAndRightEdge) -1.0))
    (Variables|Default|SetMovementVector (Math|Float|Absolute(Float) (Variables|Default|GetMovementVector)))
    (elif (> (.x (Transformation|GetWorldLocation (Variables|Default|GetDefaultSceneRoot))) (Variables|Default|GetLeftAndRightEdge))
      (Variables|Default|SetMovementVector (* (Math|Float|Absolute(Float) (Variables|Default|GetMovementVector)) -1.0)))))

(fn TryRotateRandomly
  (if (< (Math|Random|RandomFloat) (Variables|Default|GetChanceToChangeDirections))
    (bind _result (Math|Float|NegateFloat (Variables|Default|GetMovementVector))
      (:%20%20
        (Variables|Default|SetMovementVector _result)))))

(fn DropApple
  (Game|SpawnActorfromClass "/Game/ApplePicker/Blueprints/Actors/BP_Apple.BP_Apple_C" (Transformation|GetWorldTransform (Variables|Default|GetDefaultSceneRoot)) "Undefined" "MultiplyWithRoot" 0 0))