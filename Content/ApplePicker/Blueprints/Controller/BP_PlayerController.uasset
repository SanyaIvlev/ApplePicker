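; Player controller for ApplePicker that slides the active basket horizontally under the mouse cursor.
; On BeginPlay it caches the controlled basket and its camera, shows the cursor and match info widget, then possesses the last basket from GM_GameMode.
; Tick deprojects the mouse position and moves the basket along world X only.
; When a basket is destroyed, it possesses the game mode's next last basket, if any remain.
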(event Custom|OnBasketDestroyed
  (bind _game_mode (Variables|Default|GetGame%20Mode))
  (bind _last_basket (Default|GetLastBasket _game_mode))
  (Pawn|UnPossess)
  (if (not (Utilities|Array|IsEmpty (Variables|/Game/ApplePicker/Blueprints/GameMode/GM_GameMode.GM_GameMode_C|GetBaskets _game_mode)))
    (Pawn|Possess _last_basket)
    (Variables|Default|SetBasket _last_basket)))

(event EventTick
  (params (DeltaSeconds :type Float%20%28single-precision%29))
  (bind (_locationx _locationy) (Game|Player|GetMousePosition))
  (bind _basket (Variables|Default|GetBasket))
  (bind _basket_2 (Variables|Default|GetBasket))
  (bind _basket_mesh (Variables|/Game/ApplePicker/Blueprints/Pawns/BP_Basket.BP_Basket_C|GetBasket%20Mesh _basket_2))
  (bind _returnvalue (Transformation|GetWorldLocation _basket_mesh))
  (Utilities|IsValid _basket
    (:Is%20Valid
      (Default|Move _basket (Math|Vector|MakeVector (.x (.WorldLocation (Class|PlayerController|DeprojectScreenPositiontoWorld _locationx _locationy))) (.y _returnvalue) (.z _returnvalue))))))

(event EventBeginPlay
  (CallFunction|InitializeVariables)
  (Variables|Default|SetbShowMouseCursor true)
  (bind _returnvalue (Game|ConstructObjectfromClass "/Game/ApplePicker/Blueprints/Widgets/WBP_MatchInfo.WBP_MatchInfo_C"))
  (UserInterface|Viewport|AddtoViewport _returnvalue 0)
  (bind _asgm_game_mode (Utilities|Casting|CastToGM_GameMode (Game|GetGameMode)))
  (Utilities|IsValid _asgm_game_mode
    (:Is%20Valid
      (bind _output_get (Variables|Default|SetGame%20Mode _asgm_game_mode))
      (Pawn|Possess (Utilities|Array|Get(acopy) (Variables|/Game/ApplePicker/Blueprints/GameMode/GM_GameMode.GM_GameMode_C|GetBaskets _output_get) (Utilities|Array|LastIndex (Variables|/Game/ApplePicker/Blueprints/GameMode/GM_GameMode.GM_GameMode_C|GetBaskets _output_get)))))))

(fn ConstructionScript)

(fn InitializeVariables
  (bind _asbp_basket (Utilities|Casting|CastToBP_Basket (Pawn|GetControlledPawn)))
  (Utilities|IsValid _asbp_basket
    (:Is%20Valid
      (bind _output_get (Variables|Default|SetBasket _asbp_basket))
      (Variables|Default|SetPlayerCamera (Variables|/Game/ApplePicker/Blueprints/Pawns/BP_Basket.BP_Basket_C|GetCamera _output_get)))))