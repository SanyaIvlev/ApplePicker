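; Game mode for the Apple Picker game that handles losing a basket when an apple is destroyed, and the game over that follows.
; On BeginPlay it caches the player's BP_Basket pawn and the GS_GameState.
; OnAppleDestroyed clears every BP_Apple from the level and removes the last basket mesh.
; When no basket meshes remain, it saves the high score through the game state and reloads the L_ApplePicker level.
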(event Custom|OnAppleDestroyed
  (Utilities|FlowControl|Sequence
    (:then_0
      (bind _outactors (Actor|GetAllActorsOfClass "/Game/ApplePicker/Blueprints/BP_Apple.BP_Apple_C"))
      (for _array_element _outactors
        (Actor|DestroyActor _array_element)))
    (:then_1
      (CallFunction|RemoveBasket))
    (:then_2
      (if (Utilities|Array|IsEmpty (Variables|/Game/ApplePicker/Blueprints/BP_Basket.BP_Basket_C|GetBasket%20Meshes (Variables|Default|GetBasket)))
        (Default|SaveHighScore (Variables|Default|GetGame%20State))
        (Game|OpenLevel(byObjectReference) "/Game/ApplePicker/Maps/L_ApplePicker.L_ApplePicker")))))

(event EventBeginPlay
  (Utilities|FlowControl|Sequence
    (:then_0
      (bind _asbp_basket (Utilities|Casting|CastToBP_Basket (Game|Player|GetPlayerPawn 0)))
      (Utilities|IsValid _asbp_basket
        (:Is%20Valid
          (Variables|Default|SetBasket _asbp_basket))))
    (:then_1
      (bind _asgs_game_state (Utilities|Casting|CastToGS_GameState (Game|GetGameState)))
      (Utilities|IsValid _asgs_game_state
        (:Is%20Valid
          (Variables|Default|SetGame%20State _asgs_game_state))))))

(fn ConstructionScript)

(fn RemoveBasket
  (bind _basket (Variables|Default|GetBasket))
  (bind _basket_meshes (Variables|/Game/ApplePicker/Blueprints/BP_Basket.BP_Basket_C|GetBasket%20Meshes _basket))
  (bind _returnvalue (Utilities|Array|LastIndex _basket_meshes))
  (bind _output (Utilities|Array|Get(acopy) _basket_meshes _returnvalue))
  (Default|DestroyMesh (Variables|Default|GetBasket) _output)
  (Utilities|Array|RemoveItem _basket_meshes _output))