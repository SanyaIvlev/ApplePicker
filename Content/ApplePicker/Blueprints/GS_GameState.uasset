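; Game state for ApplePicker that tracks the player's score and a persistent high score.
; On BeginPlay it loads the high score from an SG_SaveGame slot, or creates a new save object if none exists.
; Each UpdateGameScore call adds a fixed increment and broadcasts the new score.
; When the score beats the high score, it updates and broadcasts the record and immediately saves it to the slot.
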(event Custom|UpdateGameScore
  (bind _output_get (Variables|Default|SetScore (+ (Variables|Default|GetScore) 100)))
  (Default|CallOnScoreUpdated _output_get)
  (if (> (Variables|Default|GetScore) (Variables|Default|GetHighScore))
    (bind _output_get_2 (Variables|Default|SetHighScore (Variables|Default|GetScore)))
    (Default|CallOnHighScoreUpdated _output_get_2)
    (CallFunction|SaveHighScore)))

(event EventBeginPlay
  (CallFunction|TryLoadHighScore))

(fn ConstructionScript)

(fn SaveHighScore
  (Variables|/Game/ApplePicker/Blueprints/SG_SaveGame.SG_SaveGame_C|SetHigh%20Score (Variables|Default|GetSaveGame) (Variables|Default|GetHighScore))
  (SaveGame|SaveGametoSlot (Variables|Default|GetSaveGame) (Variables|Default|GetSaveSlotName)))

(fn TryLoadHighScore
  (bind _returnvalue (SaveGame|DoesSaveGameExist (Variables|Default|GetSaveSlotName)))
  (if _returnvalue
    (bind _returnvalue_2 (SaveGame|LoadGamefromSlot (Variables|Default|GetSaveSlotName)))
    (bind _assg_save_game (Utilities|Casting|CastToSG_SaveGame _returnvalue_2))
    (bind _output_get (Variables|Default|SetSaveGame _assg_save_game))
    (Variables|Default|SetHighScore (Variables|/Game/ApplePicker/Blueprints/SG_SaveGame.SG_SaveGame_C|GetHigh%20Score _output_get))
    (else
      (bind _returnvalue_3 (SaveGame|CreateSaveGameObject "/Game/ApplePicker/Blueprints/SG_SaveGame.SG_SaveGame_C"))
      (Variables|Default|SetSaveGame _returnvalue_3))))